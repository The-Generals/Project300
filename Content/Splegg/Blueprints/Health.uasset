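; Health component for Splegg that tracks an owning actor's health and reports when it runs out.
; On BeginPlay it binds to the owner's point damage event and resets health to its default.
; Each hit draws a debug sphere and damage number at the impact, subtracts the damage, and sends the owner a player death message at zero or below.
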(event Custom|PointDamage
  (params (DamagedActor :type Actor%20Object%20Reference) (Damage :type Float%20%28single-precision%29) (InstigatedBy :type Controller%20Object%20Reference) (HitLocation :type Vector) (FHitComponent :type Primitive%20Component%20Object%20Reference) (BoneName :type Name) (ShotFromDirection :type Vector) (DamageType :type Damage%20Type%20Object%20Reference) (DamageCauser :type Actor%20Object%20Reference))
  (Rendering|Debug|DrawDebugSphere HitLocation 7.0 12 "(R=0.453125,G=0.000000,B=0.035606,A=1.000000)" 1.0 1.0)
  (Rendering|Debug|DrawDebugString HitLocation (Utilities|String|ToString(Float) Damage) 0 "(R=1.000000,G=1.000000,B=1.000000,A=1.000000)")
  (Variables|Default|SetHealth (- (Variables|Default|GetHealth) Damage))
  (if (<= (Variables|Default|GetHealth) 0.0)
    (Class|INTSpleggPlayer|PlayerDeath(Message) (Components|GetOwner))))

(event EventBeginPlay
  (EventDispatchers|BindEventtoOnTakePointDamage (Components|GetOwner) (delegate Custom|PointDamage))
  (Variables|Default|SetHealth (Variables|Default|GetDefaultHealth)))

(event EventTick
  (params (DeltaSeconds :type Float%20%28single-precision%29)))