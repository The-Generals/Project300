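; Player character for Splegg that picks up, equips, aims and fires weapons, with server events for multiplayer.
; Interact has the server spawn the pickup's class onto the hand socket, remove the pickup, and multicast a delayed animation and rotation switch to combat stance.
; Firing messages the weapon, with grenade launchers also spawning a server grenade.
; Aiming drives an FOV timeline and slows walk speed via server and client events.
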(event Custom|SRV_AttachWeapon
  (params (Class :type Actor%20Class%20Reference))
  (bind _self self)
  (bind _pickup (Variables|Default|GetPickup))
  (bind _returnvalue (Game|SpawnActorfromClass Class (Transformation|GetActorTransform) "AlwaysSpawn" _self _self))
  (bind _output_get (Variables|Default|SetWeapon _returnvalue))
  (Class|INTPickup|GetPlayerCamera(Message) _output_get (Variables|Default|GetCamera))
  (Transformation|AttachComponentToComponent _output_get (Variables|Character|GetMesh) "Weapon_r" "SnapToTarget" "SnapToTarget" "SnapToTarget" true)
  (Variables|Default|SetWeaponEquipped true)
  (bind _weapontype (Class|INTPickup|GetWeaponType(Message) (Variables|Default|GetPickup)))
  (Variables|Default|SetWeaponType _weapontype)
  (Class|INTPickup|DisableCollision(Message) _pickup)
  (bind _int (Default|Blendspaceint _pickup))
  (CallFunction|MultiUpdateCombatState _int)
  (Default|SRVRemovePickupfromWorld (Variables|Default|GetPickup)))

(event Custom|Multi_UpdateCombatState
  (params (Blendspaceint :type Integer))
  (bind _charactermovement (Variables|Character|GetCharacterMovement))
  (Utilities|FlowControl|Delay 1.0)
  (Class|INTAnimBPPlayer|CombatState(Message) (Components|SkeletalMesh|GetAnimInstance (Variables|Character|GetMesh)) Blendspaceint)
  (Variables|/Script/Engine.CharacterMovementComponent|SetbUseControllerDesiredRotation _charactermovement true)
  (Variables|/Script/Engine.CharacterMovementComponent|SetbOrientRotationToMovement _charactermovement false))

(event Custom|SRV_SpawnGrenade
  (Game|SpawnActorfromClass "/Game/Splegg/Pickups/Weapons/BP_LaunchedGrenade.BP_LaunchedGrenade_C" (Transformation|GetWorldTransform (Variables|Default|GetGrenadeSpawn)) "AlwaysSpawn" 0 0))

(event Custom|Client_UpdateSpeed
  (params (Speed :type Float%20%28single-precision%29))
  (Variables|/Script/Engine.CharacterMovementComponent|SetMaxWalkSpeed (Variables|Character|GetCharacterMovement) Speed))

(event Custom|SRV_UpdateSpeed
  (params (Speed :type Float%20%28single-precision%29))
  (bind _output_get (Variables|/Script/Engine.CharacterMovementComponent|SetMaxWalkSpeed (Variables|Character|GetCharacterMovement) Speed))
  (CallFunction|ClientUpdateSpeed _output_get))

(event EventBeginPlay
  (|CallParentFunction))

(event Game|Damage|EventPointDamage
  (params (Damage :type Float%20%28single-precision%29) (DamageType :type Damage%20Type%20Object%20Reference) (HitLocation :type Vector :default "0, 0, 0") (HitNormal :type Vector :default "0, 0, 0") (HitComponent :type Primitive%20Component%20Object%20Reference) (BoneName :type Name :default "None") (ShotFromDirection :type Vector :default "0, 0, 0") (InstigatedBy :type Controller%20Object%20Reference) (DamageCauser :type Actor%20Object%20Reference) (HitInfo :type Hit%20Result%20Structure%20%28by%20ref%29))
  (Rendering|Debug|DrawDebugSphere HitLocation 7.0 12 "(R=0.453125,G=0.000000,B=0.035606,A=1.000000)" 1.0 1.0))

(event EventSetPickup
  (params (Pickup :type BP%20Pickup%20Object%20Reference))
  (Variables|Default|SetPickup Pickup))

(event Input|ActionEvents|InputActionInteract
  (params (Key :type Key%20Structure :default "None"))
  (:Pressed
    (bind _pickup (Variables|Default|GetPickup)
      (:then
        (if (Variables|/Game/Splegg/Pickups/BP_Pickup.BP_Pickup_C|GetIsWeapon _pickup)
          (CallFunction|SRVAttachWeapon (Utilities|GetClass _pickup))))
      (:else))))

(event Input|ActionEvents|InputActionFireWeapon
  (params (Key :type Key%20Structure :default "None"))
  (:Pressed
    (bind _weapon (Variables|Default|GetWeapon)
      (:then
        (switch Utilities|FlowControl|Switch|SwitchonE_WeaponType (Variables|Default|GetWeaponType)
          (:NewEnumerator0
            (Class|INTPickup|FireWeapon(Message) _weapon :!label _label))
          (:NewEnumerator1
            (goto _label))
          (:NewEnumerator2
            (Class|INTPickup|FireWeapon(Message) _weapon)
            (CallFunction|SRVSpawnGrenade))))
      (:else))))

(event Input|ActionEvents|InputActionAim
  (params (Key :type Key%20Structure :default "None"))
  (bind _weaponequipped (Variables|Default|GetWeaponEquipped))
  (:Pressed
    (if _weaponequipped
      (CallFunction|SRVUpdateSpeed 2e+02)
      (bind _time (Timeline|T_FieldOfView PlayFromStart)
        (:Update
          (Camera|SetFieldOfView (Variables|Default|GetCamera) (Math|Interpolation|FInterpTo 9e+01 (Variables|Default|GetFieldOfView) _time (Math|Float|Clamp(Float) (Variables|Default|GetZoomSpeed) 0.1 1e+02)))))))
  (:Released
    (if _weaponequipped
      (CallFunction|SRVUpdateSpeed 5e+02)
      (Timeline|T_FieldOfView Reverse))))

(fn ConstructionScript
  (|CallParentFunction))

(fn SpleggPlayerRef
  (return self))