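; Base weapon pickup Blueprint that provides hitscan firing for weapons.
; A camera reference passed in through GetPlayerCamera sets the aim for SRVFireWeapon, the server-named fire event.
; Firing calls a multicast-named effects event for muzzle flash and sound, then line traces forward from the camera, ignoring owner and self.
; A hit applies point damage using the weapon's damage and damage type.
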(event Custom|Multi_WeaponEffects
  (params (EmitterTemplate :type Particle%20System%20Object%20Reference) (AttachToComponent :type Scene%20Component%20Object%20Reference) (AttachPointName :type Name))
  (Effects|SpawnEmitterAttached EmitterTemplate AttachToComponent AttachPointName)
  (Audio|PlaySoundatLocation (Variables|Default|GetWeaponFire) (Transformation|GetActorLocation) "0, 0, 0" 1.0 1.0 0.0 0 0 0))

(event EventSRVFireWeapon
  (bind _camera (Variables|Default|GetCamera))
  (CallFunction|MultiWeaponEffects (Variables|Default|GetMuzzleFlash) (Variables|Default|GetSkeletalMesh) "MuzzleFlash")
  (Variables|Default|SetCameraLocation (Transformation|GetWorldLocation _camera))
  (Variables|Default|SetCameraRotation (Transformation|GetWorldRotation _camera))
  (bind (_outhit _returnvalue) (Collision|LineTraceByChannel (Variables|Default|GetCameraLocation) (+ (Variables|Default|GetCameraLocation) (* (Math|Vector|GetForwardVector (Variables|Default|GetCameraRotation)) (Variables|Default|GetBulletDistance))) "TraceTypeQuery1" true (Utilities|Array|MakeArray (Components|GetOwner) self) "None"))
  (if _returnvalue
    (Game|Damage|ApplyPointDamage (.HitActor (Collision|BreakHitResult _outhit)) (Variables|Default|GetWeaponDamage) (Variables|Default|GetCameraLocation) _outhit (Game|GetInstigatorController) self "/Script/Engine.DamageType")))

(event EventGetPlayerCamera
  (params (PlayerCamera :type Camera%20Component%20Object%20Reference))
  (Variables|Default|SetCamera PlayerCamera))

(fn ConstructionScript
  (|CallParentFunction))