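; BP_Pickup is a weapon pickup actor in Splegg that offers itself to players who overlap its sphere.
; On authority, overlapping a "Player"-tagged actor waits briefly, then passes the pickup to that actor through SetPickupMessage.
; Server-prefixed events disable sphere collision or destroy the actor, while FireWeapon forwards to an empty server fire event.
; Getters expose its blendspace, weapon type and self reference; end overlap and the DisableCollision function do nothing.
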(event OnComponentBeginOverlap(Sphere)
  (params (OverlappedComponent :type Primitive%20Component%20Object%20Reference) (OtherActor :type Actor%20Object%20Reference) (OtherComp :type Primitive%20Component%20Object%20Reference) (OtherBodyIndex :type Integer) (bFromSweep :type Boolean) (SweepResult :type Hit%20Result%20Structure%20%28by%20ref%29))
  (Networking|SwitchHasAuthority
    (:Authority
      (if (Actor|ActorHasTag OtherActor "Player")
        (Utilities|FlowControl|Delay 0.2)
        (Class|INTSpleggPlayer|SetPickup(Message) OtherActor self)))))

(event OnComponentEndOverlap(Sphere)
  (params (OverlappedComponent :type Primitive%20Component%20Object%20Reference) (OtherActor :type Actor%20Object%20Reference) (OtherComp :type Primitive%20Component%20Object%20Reference) (OtherBodyIndex :type Integer))
  (Networking|SwitchHasAuthority))

(event Custom|SRV_RemovePickupFromWorld
  (Actor|DestroyActor))

(event Custom|SRV_DisableCollision
  (Collision|SetCollisionEnabled (Variables|Default|GetSphere) "NoCollision"))

(event Custom|SRV_FireWeapon)

(event EventFireWeapon
  (CallFunction|SRVFireWeapon))

(fn ConstructionScript)

(fn Blendspaceint
  (return (Variables|Default|GetBlendspace)))

(fn DisableCollision
  (return 0))

(fn GetWeaponType
  (return (Variables|Default|GetWeaponType)))

(fn PickupRef
  (return self))