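; Game State Blueprint that listens for player deaths and reports them with debug prints.
; On BeginPlay it prints the PlayerArray count, then binds OnDeath to the OnPlayerDeath dispatcher of each BP_PlayerState in that array.
; OnDeath prints the received player name followed by "Is Dead".
; Binding happens only at BeginPlay, so players added later are not bound here.
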(event Custom|OnDeath
  (params (PlayerName :type String))
  (Development|PrintString (Utilities|String|Append PlayerName " Is Dead")))

(event EventBeginPlay
  (Development|PrintString (Utilities|String|ToString(Integer) (Utilities|Array|Length (Variables|Default|GetPlayerArray))) true true "(R=0.579394,G=1.000000,B=0.000000,A=1.000000)")
  (for _array_element (Variables|Default|GetPlayerArray)
    (bind _asbp_player_state (Utilities|Casting|CastToBP_PlayerState _array_element))
    (EventDispatchers|AssignOnPlayerDeath _asbp_player_state (delegate Custom|OnDeath))))

(fn ConstructionScript)